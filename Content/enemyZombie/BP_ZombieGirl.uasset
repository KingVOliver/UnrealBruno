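; BP_ZombieGirl is an enemy zombie that chases and attacks the player in an FPS survival game.
; AI MoveTo targets the player controller and retries on failure, while pawn sensing raises walk speed.
; AttackPlayer uses a montage notify to damage player characters inside a sphere overlap.
; Point damage plays hit reactions or destroys the zombie; a separate Death event stops movement and decrements the game mode's enemy count.
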(event `self.ReceiveBeginPlay`
  (`self.runtoPLay`))

(event `self.ReceiveTick`
  (params (DeltaSeconds :type "Float (single-precision)")))

(event `runtoPLay`
  ;[1 1 1] movimenta inimigo
  (`|AIMoveTo` self (0.0 0.0 0.0) (`GameplayStatics.GetPlayerController` 0) 10.0
    (:`OnFail`
      (`self.runtoPLay`))))

(event `self.PawnSensing.OnSeePawn`
  (params (Pawn :type "Pawn Object Reference"))
  ;[1 1 1] muda velocidade
  (set `CharacterMovementComponent.MaxWalkSpeed` 350.0 (`self.CharacterMovement`)))

(event `AttackPlayer`
  ;[1 1 1] ataca o player
  (if (not (`self.IsDead?`))
    (`|PlayMontage` (`self.Mesh`) "/Game/Unreal5FPSSurvival-main/FPS_Files/zombieGirl/animations/attackanim.attackanim"
      (:`OnCompleted`
        (`self.runtoPLay`))
      (:`OnNotifyBegin`
        (bind (_outactors _returnvalue) (`KismetSystemLibrary.SphereOverlapActors` (`SceneComponent.K2_GetComponentLocation` (`self.Arrow1`)) 80.0 (`|MakeArray` "ObjectTypeQuery3" :!type "EObjectTypeQuery Enum") "/Game/Unreal5FPSSurvival-main/FPS_Files/Character/blueprints2/BP_FirstPersonCharacter.BP_FirstPersonCharacter_C" (`|MakeArray` self :!type "Actor Object Reference")))
        (if _returnvalue
          (for _array_element _outactors
            (`GameplayStatics.ApplyDamage` _array_element 20.0 (`self.GetController`) self "/Script/Engine.DamageType")))))))

(event `self.ReceivePointDamage`
  (params (Damage :type "Float (single-precision)") (DamageType :type "DamageType Object Reference") (HitLocation :type "Vector Structure") (HitNormal :type "Vector Structure") (HitComponent :type "PrimitiveComponent Object Reference") (BoneName :type Name) (ShotFromDirection :type "Vector Structure") (InstigatedBy :type "Controller Object Reference") (DamageCauser :type "Actor Object Reference") (HitInfo :type "HitResult Structure (by ref)"))
  ;[1 1 1] dano ao inimigo
  (if (not (`self.IsDead?`))
    (bind _output_get (set `self.Health` (- (`self.Health`) Damage)))
    (if (<= _output_get 0.0)
      (`self.K2_DestroyActor`)
      (else
        (`|PlayMontage` (`self.Mesh`) "/Game/Unreal5FPSSurvival-main/FPS_Files/zombieGirl/animations/hit.hit")))))

(event `Death`
  (set `self.IsDead?` true)
  (`NavMovementComponent.StopActiveMovement` (`self.CharacterMovement`))
  (`PrimitiveComponent.SetCollisionResponseToChannel` (`self.Mesh`) "ECC_Pawn" "ECR_Overlap")
  (bind _asgame_mode_fpssurvivel (cast `/Game/FirstPerson/Blueprints/GameModeFPSSurvivel` (`GameplayStatics.GetGameMode`)))
  (`/Game/FirstPerson/Blueprints/GameModeFPSSurvivel.DecEnemies` _asgame_mode_fpssurvivel))

(fn `UserConstructionScript`)